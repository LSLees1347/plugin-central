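; BP_GlobalTime keeps a running game clock that clients smooth toward a server-side target time.
; Every tick adds delta seconds to Time; the server copies the result into Target.
; Clients interpolate Time toward Target with FInterpTo to absorb drift gradually instead of snapping.
; An unconnected debug print would show both times and their difference.
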(event EventTick
  (params (DeltaSeconds :type Float%20%28single-precision%29))
  (Variables|Default|SetTime (+ (Variables|Default|GetTime) DeltaSeconds))
  (if (Networking|IsServer)
    (bind _output_get (Variables|Default|SetTarget (Variables|Default|GetTime)))
    (else
      (bind _output_get_2 (Variables|Default|SetTime (Math|Interpolation|FInterpTo (Variables|Default|GetTime) (Variables|Default|GetTarget) DeltaSeconds 1.0))))))

(fn ConstructionScript)